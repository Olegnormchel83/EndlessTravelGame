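; Enemy spawner actor that keeps its area populated with enemies up to a maximum count.
; A looping timer, cleared on EndPlay, spawns one enemy per check at random XY within the SpawnBorder box and passes it a random level and spawn location.
; Colliding spawns are adjusted or skipped, and each spawned enemy's OnDied event decrements the count to free a slot.
; Tick prints the current count on screen.
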(event Custom|CheckEnemiesCount
  (bind _spawnborder (Variables|Default|GetSpawnBorder))
  (bind _spawnborder_2 (Variables|Default|GetSpawnBorder))
  (bind _returnvalue (Transformation|GetWorldLocation _spawnborder_2))
  (bind _returnvalue_2 (Components|Box|GetScaledBoxExtent _spawnborder))
  (bind _returnvalue_3 (Math|Random|RandomPointinBoundingBox (Math|Vector|MakeVector (.x _returnvalue) (.y _returnvalue) (.z _returnvalue)) _returnvalue_2))
  (bind _returnvalue_4 (Math|Vector|MakeVector (.x _returnvalue_3) (.y _returnvalue_3) (.z _returnvalue)))
  (if (< (Variables|Default|GetCurrentEnemiesCount) (Variables|Settings|GetMaxEnemiesCount))
    (bind _returnvalue_5 (Game|SpawnActorfromClass (Variables|Settings|GetEnemyClass) (Math|Transform|MakeTransform _returnvalue_4) "AdjustIfPossibleButDontSpawnIfColliding" "MultiplyWithRoot" 0 (Math|Random|RandomIntegerinRange (Variables|Settings|GetMinLevel) (Variables|Settings|GetMaxLevel)) _returnvalue_4 0))
    (Utilities|IsValid _returnvalue_5
      (:Is%20Valid
        (bind _result (Math|Integer|IncrementInt (Variables|Default|GetCurrentEnemiesCount))
          (:%20%20
            (Variables|Default|SetCurrentEnemiesCount _result)
            (EventDispatchers|BindEventtoOnDied _returnvalue_5 (delegate Custom|OnSpawnedEnemyDied_Event))))))))

(event Custom|OnSpawnedEnemyDied_Event
  (bind _result (Math|Integer|DecrementInt (Variables|Default|GetCurrentEnemiesCount))
    (:%20%20
      (Variables|Default|SetCurrentEnemiesCount _result))))

(event EventBeginPlay
  (bind _returnvalue (Utilities|Time|SetTimerbyEvent (delegate Custom|CheckEnemiesCount) (Variables|Settings|GetCheckEnemiesCountTimer) true))
  (Variables|Default|SetSpawnerTimerHandle _returnvalue))

(event EventEndPlay
  (params (EndPlayReason :type EEndPlayReason%20Enum :default "Destroyed"))
  (bind _spawnertimerhandle (Variables|Default|GetSpawnerTimerHandle))
  (if (Utilities|Time|IsValidTimerHandle _spawnertimerhandle)
    (Utilities|Time|ClearandInvalidateTimerbyHandle _spawnertimerhandle)))

(event EventTick
  (params (DeltaSeconds :type Float%20%28single-precision%29))
  (Development|PrintString (Utilities|String|Append "Current Enemies Count: " (Utilities|String|ToString(Integer) (Variables|Default|GetCurrentEnemiesCount))) true false "(R=0.000000,G=0.660000,B=1.000000,A=1.000000)" 0.0))

(fn ConstructionScript)