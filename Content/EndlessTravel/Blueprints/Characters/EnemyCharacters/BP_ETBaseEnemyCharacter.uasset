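; Base enemy character for EndlessTravel that holds an AI state, follows health changes and supplies patrol points.
; ChangeState sets walk speed for Chase, Patrol and Attention.
; Health changes read an Ability System attribute; at zero or below the enemy ragdolls, drops capsule collision, removes its widget and gets a short life span.
; GetNextPointOnPatrolRoute cycles through the patrol route's spline points in world space, wrapping at the end.
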(event Custom|OnDied_Event
  (bind _mesh (Variables|Character|GetMesh))
  (Variables|Default|SetbIsAlive false)
  (Physics|SetSimulatePhysics _mesh true)
  (Collision|SetCollisionProfileName _mesh "Ragdoll" true :!class /Script/Engine.PrimitiveComponent)
  (Collision|SetCollisionEnabled (Variables|Default|GetCapsuleComponent) "NoCollision")
  (Actor|SetLifeSpan 5.0)
  (bind _widget (Variables|Default|GetWidget)
    (:then
      (Components|DestroyComponent _widget))
    (:else)))

(event EventBeginPlay
  (|CallParentFunction)
  (Variables|Default|SetbIsAlive true))

(event Collision|EventActorBeginOverlap
  (params (OtherActor :type Actor%20Object%20Reference)))

(event EventTick
  (params (DeltaSeconds :type Float%20%28single-precision%29)))

(event EventChangeState
  (params (InState :type E_EnemyState%20Enum :default "NewEnumerator0"))
  (bind _output_get (Variables|Default|SetState InState))
  (Variables|Character|GetCharacterMovement
    (:then
      (switch Utilities|FlowControl|Switch|SwitchonE_EnemyState _output_get
        (:NewEnumerator0
          (Variables|/Script/Engine.CharacterMovementComponent|SetMaxWalkSpeed (Variables|Character|GetCharacterMovement) 6e+02))
        (:NewEnumerator1
          (Variables|/Script/Engine.CharacterMovementComponent|SetMaxWalkSpeed (Variables|Character|GetCharacterMovement) 1.5e+02))
        (:NewEnumerator2
          (Variables|/Script/Engine.CharacterMovementComponent|SetMaxWalkSpeed (Variables|Character|GetCharacterMovement) 3e+02))))
    (:else)))

(event EventOnHealthChangedEvent
  (if (Variables|Default|GetbIsAlive)
    (Default|CallOnHealthChanged)
    (if (<= (.ReturnValue (Ability|Attribute|GetFloatAttributefromAbilitySystemComponent (Variables|Default|GetAbilitySystem) "(AttributeName=\"Health\",Attribute=/Script/EndlessTravel.ET_BaseAttributeSet:Health,AttributeOwner=\"/Script/CoreUObject.Class'/Script/EndlessTravel.ET_BaseAttributeSet'\")")) 0.0)
      (Default|CallOnDied)
      (CallFunction|OnDiedEvent))))

(fn ConstructionScript
  (|CallParentFunction))

(fn GetAbilitySystem
  (return 0))

(fn GetNextPointonPatrolRoute
  (bind _patrolroute (Variables|Settings|GetPatrolRoute)
    (:then
      (bind _output_get (Variables|Default|SetLastPointIndex (Math|Integer|%(Integer) (+ (Variables|Default|GetLastPointIndex) 1) (Spline|GetNumberOfSplinePoints (Variables|/Game/EndlessTravel/Blueprints/Characters/EnemyCharacters/OrdinaryCorpse/BP_PatrolRoute.BP_PatrolRoute_C|GetSpline _patrolroute)))))
      (return (Spline|GetLocationatSplinePoint (Variables|/Game/EndlessTravel/Blueprints/Characters/EnemyCharacters/OrdinaryCorpse/BP_PatrolRoute.BP_PatrolRoute_C|GetSpline _patrolroute) _output_get "World") (Variables|Default|GetLastPointIndex)))
    (:else
      (return "0, 0, 0" (Variables|Default|GetLastPointIndex)))))

(fn GetShouldTrace
  (return false))

(fn GetSkeletalMesh
  (return 0))

(fn GetSpawnLocation
  (return (Variables|Settings|GetSpawnLocation)))

(fn GetState
  (return (Variables|Default|GetState)))

(fn IsAlive
  (return (Variables|Default|GetbIsAlive)))