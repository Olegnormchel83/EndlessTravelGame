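; AI controller for the Ordinary Corpse enemy that runs its behavior tree on possess and reacts to AI perception.
; Seeing the player stores the target and sets PlayerInTarget on the Blackboard.
; Losing sight starts a timer from the stimulus expiration age to forget the player, cancelled if the player is seen again.
; Hearing the player writes LocationToInvestigate, but only while the pawn is in a specific state.
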(event OnTargetPerceptionUpdated(AIPerception)
  (params (Actor :type Actor%20Object%20Reference) (Stimulus :type AI%20Stimulus%20Structure))
  (bind _returnvalue (Class|AIPerceptionSystem|GetSenseClassforStimulus Stimulus))
  (Utilities|FlowControl|Sequence
    (:then_0
      (if (== _returnvalue "/Script/AIModule.AISense_Sight")
        (CallFunction|SightReaction Actor Stimulus)))
    (:then_1
      (if (== _returnvalue "/Script/AIModule.AISense_Hearing")
        (CallFunction|HearingReaction Actor Stimulus)))))

(event EventBeginPlay)

(event EventTick
  (params (DeltaSeconds :type Float%20%28single-precision%29)))

(event EventPossess
  (params (PossessedPawn :type Pawn%20Object%20Reference))
  (AI|RunBehaviorTree "/Game/EndlessTravel/Blueprints/Characters/EnemyCharacters/OrdinaryCorpse/BT_OrdinaryCorpse.BT_OrdinaryCorpse"))

(fn ConstructionScript
  (|CallParentFunction))

(fn GetTargetActor
  (bind _targetactor (Variables|Default|GetTargetActor))
  (Utilities|IsValid _targetactor
    (:Is%20Valid
      (return _targetactor))
    (:Is%20Not%20Valid
      (return 0))))

(fn GetLastStimulusLocation
  (return (Variables|Default|GetSight%20Stimulus%20Location)))

(fn SightReaction
  (params (TargetActor :type Actor%20Object%20Reference) (AIStimulus :type AI%20Stimulus%20Structure%20%28by%20ref%29))
  (bind (_age _expirationage _strength _stimuluslocation _receiverlocation _tag _bsuccessfullysensed) (Utilities|Struct|BreakAIStimulus AIStimulus))
  (if (CallFunction|IsPlayer TargetActor)
    (if _bsuccessfullysensed
      (Utilities|FlowControl|Sequence
        (:then_0
          (Development|PrintString "Увидел игрока" true false)
          (Variables|Default|SetTargetActor TargetActor))
        (:then_1
          (AI|Components|Blackboard|SetValueasBool (AI|GetBlackboard 0) (Utilities|Name|MakeLiteralName "PlayerInTarget") true)
          (if (Utilities|Time|IsTimerActivebyHandle (Variables|Default|GetForgotPlayerTimerHandle))
            (Utilities|Time|ClearandInvalidateTimerbyHandle (Variables|Default|GetForgotPlayerTimerHandle))
            (Development|PrintString "Таймер закрыт" true false))))
      (else
        (bind _returnvalue (Utilities|Time|SetTimerbyEvent (EventDispatchers|CreateEvent :!event ForgetPlayer) _expirationage))
        (Variables|Default|SetForgotPlayerTimerHandle _returnvalue)
        (Development|PrintString "Начинаем забывать игрока" true false)))))

(fn ForgetPlayer
  (bind _returnvalue (AI|GetBlackboard 0))
  (AI|Components|Blackboard|SetValueasBool _returnvalue (Utilities|Name|MakeLiteralName "PlayerInTarget") false)
  (AI|Components|Blackboard|ClearValue _returnvalue (Utilities|Name|MakeLiteralName "PlayerLocation"))
  (Development|PrintString "Забыли игрока" true false))

(fn HearingReaction
  (params (TargetActor :type Actor%20Object%20Reference) (AIStimulus :type AI%20Stimulus%20Structure))
  (bind (_age _expirationage _strength _stimuluslocation _receiverlocation _tag _bsuccessfullysensed) (Utilities|Struct|BreakAIStimulus AIStimulus))
  (bind _state (Class|BPIEnemy|GetState(Message) (Pawn|GetControlledPawn)))
  (if (Utilities|Enum|Equal(Enum) _state "NewEnumerator1")
    (if (and (CallFunction|IsPlayer TargetActor) _bsuccessfullysensed)
      (AI|Components|Blackboard|SetValueasVector (Variables|Default|GetBlackboard) (Utilities|Name|MakeLiteralName "LocationToInvestigate") _stimuluslocation))))