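; Blueprint for the Ordinary Corpse enemy character in EndlessTravel, a thin child that leaves most behavior to its parent class.
; Tick calls the parent, then prints the current State enum on screen every frame as a debug readout.
; GetSkeletalMesh returns the character's Mesh component, while the construction script only calls the parent and BeginPlay and overlap events are disabled stubs.
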(event EventBeginPlay
  (|CallParentFunction) ; This node is disabled and will not be called.\nDrag off pins to build functionality.
)

(event Collision|EventActorBeginOverlap
  (params (OtherActor :type Actor%20Object%20Reference))
  (|CallParentFunction OtherActor) ; This node is disabled and will not be called.\nDrag off pins to build functionality.
)

(event EventTick
  (params (DeltaSeconds :type Float%20%28single-precision%29))
  (|CallParentFunction DeltaSeconds)
  (Development|PrintString (Utilities|String|Append "CurrentState: " (Utilities|String|EnumtoString (Variables|Default|GetState))) true false "(R=0.000000,G=0.660000,B=1.000000,A=1.000000)" 0.0))

(fn ConstructionScript
  (|CallParentFunction))

(fn GetSkeletalMesh
  (return (Variables|Character|GetMesh)))