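; Base player character Blueprint for Endless Travel, built on the Gameplay Ability System.
; On BeginPlay it grants Shoot, Sprint and Stealth abilities with input IDs, stores their handles, applies a passive ST recovery effect and tags itself as a player.
; Helper functions report sprinting from a gameplay tag and forward running from a velocity-to-facing dot product.
; Several getters, including mesh, materials and tag container, return nothing here.
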(event EventBeginPlay
  (Utilities|FlowControl|Sequence
    (:then_0
      ;[1 1 1] Shoot
      (bind _returnvalue (GameplayAbilities|GiveAbility (Variables|Default|GetAbilitySystem) "/Game/EndlessTravel/GAS/Abilities/Shoot/GA_Shoot.GA_Shoot_C" 0 1))
      (Utilities|Map|Add (Variables|Abilities|GetAbilities) 0 _returnvalue)
      ;[1 1 1] Sprint
      (bind _returnvalue_2 (GameplayAbilities|GiveAbility (Variables|Default|GetAbilitySystem) "/Game/EndlessTravel/GAS/Abilities/Sprint/GA_Sprint.GA_Sprint_C" 0 2))
      (Utilities|Map|Add (Variables|Abilities|GetAbilities) 1 _returnvalue_2)
      ;[1 1 1] Stealth
      (bind _returnvalue_3 (GameplayAbilities|GiveAbility (Variables|Default|GetAbilitySystem) "/Game/EndlessTravel/GAS/Abilities/Stealth/GA_Stealth.GA_Stealth_C" 0 3))
      (Utilities|Map|Add (Variables|Abilities|GetAbilities) 2 _returnvalue_3))
    (:then_1
      (GameplayEffects|ApplyGameplayEffectToSelf :self (Variables|Default|GetAbilitySystem) :GameplayEffectClass "/Game/EndlessTravel/GAS/Abilities/PassiveEffects/GE_PassiveSTRecovery.GE_PassiveSTRecovery_C" :Level 1.0))
    (:then_2
      (GameplayTags|AddGameplayTag (Variables|Default|GetTag%20Container) "(TagName=\"Entity.Player\")" :!class /Script/GameplayTags.BlueprintGameplayTagLibrary))))

(fn ConstructionScript
  (|CallParentFunction))

(fn IsRunForward
  (bind _charactermovement (Variables|Character|GetCharacterMovement)
    (:then
      (return (Math|Float|NearlyEqual(Float) (Math|Vector|DotProduct (Math|Vector|Normalize (Variables|/Script/Engine.MovementComponent|GetVelocity _charactermovement) 1.0) (Transformation|GetActorForwardVector)) 1.0 0.5)))
    (:else)))

(fn IsSprinting
  (bind _abilitysystem (Variables|Default|GetAbilitySystem)
    (:then
      (return (GameplayTags|HasMatchingGameplayTag _abilitysystem "(TagName=\"Status.Character.Sprinting\")")))
    (:else
      (return false))))

(fn GetCamera
  (return (Variables|Default|GetCamera)))

(fn GetCharacterMovement
  (return 0))

(fn GetDefaultMaterials
  (return 0))

(fn GetPlayerClass)

(fn GetSkeletalMesh
  (return 0))

(fn GetTagContainer
  (return ""))