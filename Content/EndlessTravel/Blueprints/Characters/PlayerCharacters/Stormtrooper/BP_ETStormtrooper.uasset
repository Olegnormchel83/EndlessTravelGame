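; Stormtrooper player character for EndlessTravel, built on the Gameplay Ability System.
; BeginPlay caches mesh materials, sets the player class, applies startup effects, and grants the reload ability.
; Passive health regen is a SetByCaller effect, scaled from MaxHealth and regen percent in the base-attribute curve table.
; Reload input activates the ability unless an attribute check finds it unnecessary, health depletion calls Dead, and a ground physical-material trace sits unused.
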(event Input|EnhancedActionEvents|EnhancedInputActionIA_ETReload
  (params (ActionValue :type Boolean) (ElapsedSeconds :type Float%20%28double-precision%29) (TriggeredSeconds :type Float%20%28double-precision%29) (InputAction :type Input%20Action%20Object%20Reference :default "/Game/EndlessTravel/Core/EnhancedInput/Actions/IA_ETReload.IA_ETReload"))
  (bind _abilitysystem (Variables|Default|GetAbilitySystem))
  (bind _abilities (Variables|Default|GetAbilities))
  (bind (_value _returnvalue) (Utilities|Map|Find _abilities 3))
  (:Started
    (if (== (.ReturnValue (Ability|Attribute|GetFloatAttributefromAbilitySystemComponent _abilitysystem "(AttributeName=\"CurrentPatronsCount\",Attribute=/Script/EndlessTravel.ET_BaseAttributeSet:CurrentPatronsCount,AttributeOwner=\"/Script/CoreUObject.Class'/Script/EndlessTravel.ET_BaseAttributeSet'\")")) (.ReturnValue (Ability|Attribute|GetFloatAttributefromAbilitySystemComponent _abilitysystem "(AttributeName=\"MaxPatronsCount\",Attribute=/Script/EndlessTravel.ET_BaseAttributeSet:MaxPatronsCount,AttributeOwner=\"/Script/CoreUObject.Class'/Script/EndlessTravel.ET_BaseAttributeSet'\")")))
      (Development|PrintString "Перезарядка не требуеся" true false)
      (elif _returnvalue
        (Class|AbilitySystemComponent|TryActivateAbility (Variables|Default|GetAbilitySystem) _value true)))))

(event EventBeginPlay
  (|CallParentFunction)
  (Utilities|FlowControl|Sequence
    (:then_0
      (Variables|Default|SetDefaultMaterials (Rendering|Material|GetMaterials (Variables|Character|GetMesh)))
      (Variables|Default|SetPlayerClass "NewEnumerator0"))
    (:then_1
      (for _array_element (Variables|Default|GetEffects)
        (if (Utilities|IsValidClass _array_element)
          (GameplayEffects|ApplyGameplayEffectToSelf (Variables|Default|GetAbilitySystem) _array_element 1.0 (GameplayEffects|MakeEffectContext (Variables|Default|GetAbilitySystem))))))
    (:then_2
      (bind _outxy (DataTable|EvaluateCurveTableRow "/Game/EndlessTravel/Blueprints/Characters/PlayerCharacters/Stormtrooper/CT_StormtrooperBaseAttributes.CT_StormtrooperBaseAttributes" "MaxHealth")
        (:RowFound
          (bind _outxy_2 (DataTable|EvaluateCurveTableRow "/Game/EndlessTravel/Blueprints/Characters/PlayerCharacters/Stormtrooper/CT_StormtrooperBaseAttributes.CT_StormtrooperBaseAttributes" "HealthRegenPercent")
            (:RowFound
              (bind _returnvalue (Ability|GameplayEffect|AssignTagSetbyCallerMagnitude (GameplayEffects|MakeOutgoingSpec :self (Variables|Default|GetAbilitySystem) :GameplayEffectClass "/Game/EndlessTravel/GAS/Abilities/PassiveEffects/GE_PassiveHPRecovery.GE_PassiveHPRecovery_C" :Level 1.0) "(TagName=\"Effect.Passive.Regen.Health.Value\")" (* _outxy _outxy_2)))
              (GameplayEffects|ApplyGameplayEffectSpecToSelf (Variables|Default|GetAbilitySystem) _returnvalue))))))
    (:then_3
      (bind _returnvalue_2 (GameplayAbilities|GiveAbility (Variables|Default|GetAbilitySystem) "/Game/EndlessTravel/GAS/Abilities/Reload/GA_StormtrooperReload.GA_StormtrooperReload_C" 0 -1))
      (Utilities|Map|Add (Variables|Default|GetAbilities) 3 _returnvalue_2))))

(event EventHPChanged
  (if (<= (.ReturnValue (Class|AbilitySystemBlueprintLibrary|GetFloatAttributeBasefromAbilitySystemComponent (Variables|Default|GetAbilitySystem) "(AttributeName=\"Health\",Attribute=/Script/EndlessTravel.ET_BaseAttributeSet:Health,AttributeOwner=\"/Script/CoreUObject.Class'/Script/EndlessTravel.ET_BaseAttributeSet'\")")) 0.0)
    (CallFunction|Dead)))

(fn ConstructionScript
  (|CallParentFunction))

(fn GetCharacterMovement
  (return (Variables|Character|GetCharacterMovement)))

(fn GetSkeletalMesh
  (return (Variables|Character|GetMesh)))

(fn GetDefaultMaterials
  (return (Variables|Default|GetDefaultMaterials)))

(fn GetTagContainer
  (return (Variables|Default|GetTag%20Container)))

(fn GetPlayerClass
  (return (Variables|Default|GetPlayerClass)))