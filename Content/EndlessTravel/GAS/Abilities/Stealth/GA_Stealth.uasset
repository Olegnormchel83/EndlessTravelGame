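; Gameplay Ability that puts the avatar into stealth, swapping every mesh material for a stealth material and slowing its walk speed.
; Activation reaches mesh and movement through BPI_GASHelper, cancelling without it, and applies duration, cost and cooldown effects directly.
; An attribute value sets both the SetByCaller duration and a timer.
; Ending restores default materials and walk speed, removing the duration effect if cancelled.
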(event Ability|EventActivateAbility
  (bind _returnvalue (Ability|GetAvatarActorfromActorInfo))
  (bind _returnvalue_2 (Ability|GetAbilitySystemComponent _returnvalue))
  (bind _returnvalue_3 (Class|AbilitySystemBlueprintLibrary|GetFloatAttributeBasefromAbilitySystemComponent _returnvalue_2 "(AttributeName=\"StealthDuration\",Attribute=/Script/EndlessTravel.ET_BaseAttributeSet:StealthDuration,AttributeOwner=\"/Script/CoreUObject.Class'/Script/EndlessTravel.ET_BaseAttributeSet'\")"))
  (Utilities|FlowControl|Sequence
    (:then_0
      (Development|PrintString "Stealth ability begin" true false))
    (:then_1
      (if (Utilities|DoesObjectImplementInterface _returnvalue "/Game/EndlessTravel/Blueprints/Interfaces/BPI_GASHelper.BPI_GASHelper_C")
        (bind _skeletalmesh (Class|BPIGASHelper|GetSkeletalMesh(Message) _returnvalue))
        (for (_ _array_index) (Rendering|Material|GetMaterials _skeletalmesh)
          (Rendering|Material|SetMaterial _skeletalmesh _array_index (Variables|Default|GetStealthMaterial)))
        (bind _returnvalue_4 (Ability|GameplayEffect|AssignTagSetbyCallerMagnitude (Ability|MakeOutgoingGameplayEffectSpec "/Game/EndlessTravel/GAS/Abilities/Stealth/GE_StealthDuration.GE_StealthDuration_C") "(TagName=\"Effect.Ability.Stealth.Duration\")" _returnvalue_3))
        (bind _returnvalue_5 (Ability|ApplyGameplayEffectSpecToOwner _returnvalue_4))
        (Variables|Default|SetStealthDurationEffect _returnvalue_5)
        (Ability|ApplyGameplayEffectToOwner "/Game/EndlessTravel/GAS/Abilities/Stealth/GE_StealthCost.GE_StealthCost_C")
        (Ability|ApplyGameplayEffectToOwner "/Game/EndlessTravel/GAS/Abilities/Stealth/GE_StealthCooldown.GE_StealthCooldown_C")
        (Utilities|FlowControl|Sequence
          (:then_0
            (Development|PrintString "Stealth go cd" true false))
          (:then_1
            (bind _charactermovement (Class|BPIGASHelper|GetCharacterMovement(Message) _returnvalue))
            (Variables|/Script/Engine.CharacterMovementComponent|SetMaxWalkSpeed _charactermovement 3e+02)
            (Utilities|Time|SetTimerbyEvent (EventDispatchers|CreateEvent :!event K2EndAbility) _returnvalue_3)))
        (else
          (Ability|CancelAbility))))))

(event Ability|EventOnEndAbility
  (params (bWasCancelled :type Boolean))
  (bind _returnvalue (Ability|GetAvatarActorfromActorInfo))
  (if bWasCancelled
    (Ability|RemoveGameplayEffectFromOwnerWithHandle (Variables|Default|GetStealthDurationEffect)))
  (Development|PrintString "Stealth ability end" true false)
  (bind _newparam (Class|BPIGASHelper|GetDefaultMaterials(Message) _returnvalue))
  (for (_ _array_index) _newparam
    (Rendering|Material|SetMaterial (stale Ability|EventActivateAbility _skeletalmesh) _array_index (Utilities|Array|Get(acopy) _newparam _array_index))
    (bind _charactermovement (Class|BPIGASHelper|GetCharacterMovement(Message) _returnvalue))
    (Variables|/Script/Engine.CharacterMovementComponent|SetMaxWalkSpeed _charactermovement 6e+02)))