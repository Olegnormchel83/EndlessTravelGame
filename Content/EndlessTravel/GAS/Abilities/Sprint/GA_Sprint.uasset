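; Gameplay Ability that lets a BP_ETBaseCharacter sprint while the input is held, by raising its max walk speed.
; A WaitDelay loop commits the ability cost every tick of a short interval for as long as the character keeps moving.
; Input release, a failed cost commit or near-zero velocity calls CustomEndAbility, which restores walk speed and ends the ability.
; OnEndAbility is unused, so speed resets only through that function.
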(event Ability|EventActivateAbility
  (bind _asbp_etbase_character (Utilities|Casting|CastToBP_ETBaseCharacter (Ability|GetAvatarActorfromActorInfo))
    (:then
      (Variables|Default|SetAvatarCharacter _asbp_etbase_character)
      (Ability|Tasks|WaitInputRelease false
        (:then
          (bind _returnvalue (Ability|CommitAbilityCost false :!label _label))
          (if _returnvalue
            (Variables|/Script/Engine.CharacterMovementComponent|SetMaxWalkSpeed (Variables|/Script/Engine.Character|GetCharacterMovement (Variables|Default|GetAvatarCharacter)) 9e+02)
            (if (not (Math|Vector|VectorIsNearlyZero (Variables|/Script/Engine.MovementComponent|GetVelocity (Variables|/Script/Engine.Character|GetCharacterMovement (Variables|Default|GetAvatarCharacter)))))
              (Ability|Tasks|WaitDelay 0.1
                (:OnFinish
                  (goto _label)))
              (else
                (CallFunction|CustomEndAbility)))
            (else
              (CallFunction|CustomEndAbility))))
        (:OnRelease
          (CallFunction|CustomEndAbility))))
    (:CastFailed
      (Ability|CancelAbility))))

(event Ability|EventOnEndAbility
  (params (bWasCancelled :type Boolean)))

(fn CustomEndAbility
  (Variables|/Script/Engine.CharacterMovementComponent|SetMaxWalkSpeed (Variables|/Script/Engine.Character|GetCharacterMovement (Variables|Default|GetAvatarCharacter)) 6e+02)
  (Ability|EndAbility))