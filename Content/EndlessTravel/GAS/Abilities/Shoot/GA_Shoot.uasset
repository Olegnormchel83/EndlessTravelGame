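; Gameplay ability for hitscan automatic weapon fire, repeating after an attribute-driven delay until input is released.
; Each shot traces from the camera over an attribute-driven range, cancelling if the hit is closer than the muzzle or the cost cannot be committed.
; It plays a class-specific gameplay cue (Stormtrooper, Sniper, Medic) and applies GE_Damage to ability-system targets via SetByCaller, with a large headshot multiplier.
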(event Ability|EventActivateAbility
  (bind _returnvalue (Ability|GetAvatarActorfromActorInfo))
  (bind _returnvalue_2 (Ability|GetAvatarActorfromActorInfo))
  (bind _returnvalue_3 (Ability|GetAbilitySystemComponent _returnvalue_2))
  (bind _returnvalue_4 (Ability|Attribute|GetFloatAttributefromAbilitySystemComponent _returnvalue_3 "(AttributeName=\"WeaponDamage\",Attribute=/Script/EndlessTravel.ET_BaseAttributeSet:WeaponDamage,AttributeOwner=\"/Script/CoreUObject.Class'/Script/EndlessTravel.ET_BaseAttributeSet'\")"))
  (bind _returnvalue_5 (* _returnvalue_4 -1.0))
  (Ability|Tasks|WaitInputRelease false
    (:then
      (if (Utilities|DoesObjectImplementInterface _returnvalue "/Game/EndlessTravel/Blueprints/Interfaces/BPI_GASHelper.BPI_GASHelper_C") :!label _label
        (bind _skeletalmesh (Class|BPIGASHelper|GetSkeletalMesh(Message) _returnvalue))
        (bind _camera (Class|BPIGASHelper|GetCamera(Message) _returnvalue))
        (bind _outhit (Collision|LineTraceByChannel (Transformation|GetWorldLocation _camera) (+ (Transformation|GetWorldLocation _camera) (* (Math|Vector|GetForwardVector _camera) (.ReturnValue (Ability|Attribute|GetFloatAttributefromAbilitySystemComponent (Ability|GetAbilitySystemComponent _returnvalue) "(AttributeName=\"WeaponDistance\",Attribute=/Script/EndlessTravel.ET_BaseAttributeSet:WeaponDistance,AttributeOwner=\"/Script/CoreUObject.Class'/Script/EndlessTravel.ET_BaseAttributeSet'\")")))) "TraceTypeQuery3" false 0 "ForDuration"))
        (if (.bBlockingHit (Collision|BreakHitResult _outhit))
          (if (< (.Distance (Collision|BreakHitResult _outhit)) (Math|Vector|Distance(Vector) (Transformation|GetWorldLocation _camera) (Transformation|GetSocketLocation _skeletalmesh "Muzzle")))
            (Development|PrintString "Shooting range is too small" true false "(R=1.000000,G=0.000000,B=0.015508,A=1.000000)")
            (Ability|CancelAbility)
            (else
              (bind _returnvalue_6 (Ability|CommitAbilityCost false :!label _label_2))
              (if _returnvalue_6
                (bind _playerclass (Class|BPIGASHelper|GetPlayerClass(Message) (Ability|GetAvatarActorfromActorInfo)))
                (GameplayCue|ExecuteGameplayCue :GameplayCueTag (Utilities|Select :Index _playerclass :NewEnumerator0 "(TagName=\"GameplayCue.StormtrooperShoot\")" :NewEnumerator1 "(TagName=\"GameplayCue.SniperShoot\")" :NewEnumerator2 "(TagName=\"GameplayCue.MedicShoot\")"))
                (Utilities|IsValid (.HitActor (Collision|BreakHitResult _outhit))
                  (:Is%20Valid
                    (Utilities|IsValid (Ability|GetAbilitySystemComponent (.HitActor (Collision|BreakHitResult _outhit)))
                      (:Is%20Valid
                        (if (== (.HitBoneName (Collision|BreakHitResult _outhit)) "Bip001-Head")
                          (Variables|Default|SetDamageMagnitude (* _returnvalue_5 1e+02))
                          (else
                            (Variables|Default|SetDamageMagnitude _returnvalue_5)))
                        (bind _returnvalue_7 (Ability|GameplayEffect|AssignTagSetbyCallerMagnitude (GameplayEffects|MakeOutgoingSpec _returnvalue_3 "/Game/EndlessTravel/GAS/Abilities/Shoot/GE_Damage.GE_Damage_C" 1.0 (GameplayEffects|MakeEffectContext _returnvalue_3)) "(TagName=\"Effect.Ability.Shoot.Damage\")" (Variables|Default|GetDamageMagnitude)))
                        (GameplayEffects|ApplyGameplayEffectSpecToSelf (Ability|GetAbilitySystemComponent (.HitActor (Collision|BreakHitResult _outhit))) _returnvalue_7)
                        (Class|BPIEnemy|OnHealthChangedEvent(Message) (.HitActor (Collision|BreakHitResult _outhit))))
                      (:Is%20Not%20Valid
                        _))
                    (Utilities|FlowControl|Sequence
                      (:then_1
                        _)))
                  (:Is%20Not%20Valid
                    _))
                (Ability|Tasks|WaitDelay (/ (.ReturnValue (Ability|Attribute|GetFloatAttributefromAbilitySystemComponent (Ability|GetAbilitySystemComponent (Ability|GetAvatarActorfromActorInfo)) "(AttributeName=\"FireRate\",Attribute=/Script/EndlessTravel.ET_BaseAttributeSet:FireRate,AttributeOwner=\"/Script/CoreUObject.Class'/Script/EndlessTravel.ET_BaseAttributeSet'\")")) 3.6e+03)
                  (:OnFinish
                    (goto _label)))
                (else
                  (Ability|CancelAbility)))))
          (else
            (goto _label_2)))
        (else
          (Ability|CancelAbility))))
    (:OnRelease
      (Ability|EndAbility))))

(event Ability|EventOnEndAbility
  (params (bWasCancelled :type Boolean)))