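; Base player character for EndlessTravel, built on the Gameplay Ability System.
; On BeginPlay it grants shoot and sprint abilities with input IDs, stores their handles in a map, and applies a stamina recovery effect to itself.
; Shoot activates the stored shoot ability and prints debug output.
; Helper queries report sprinting via a gameplay tag and roughly forward movement via a velocity-to-facing dot product.
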(event EventBeginPlay
  (Utilities|FlowControl|Sequence
    (:then_0
      (bind _returnvalue (GameplayAbilities|GiveAbility (Variables|Default|GetAbilitySystem) "/Game/EndlessTravel/GAS/Abilities/Shoot/GA_Shoot.GA_Shoot_C" 0 1))
      (Utilities|Map|Add (Variables|Abilities|GetAbilities) 0 _returnvalue)
      (bind _returnvalue_2 (GameplayAbilities|GiveAbility (Variables|Default|GetAbilitySystem) "/Game/EndlessTravel/GAS/Abilities/Sprint/GA_Sprint.GA_Sprint_C" 0 2))
      (Utilities|Map|Add (Variables|Abilities|GetAbilities) 1 _returnvalue_2))
    (:then_1
      (GameplayEffects|ApplyGameplayEffectToSelf :self (Variables|Default|GetAbilitySystem) :GameplayEffectClass "/Game/EndlessTravel/GAS/Abilities/PassiveEffects/GE_StaminaRecovery.GE_StaminaRecovery_C"))))

(fn ConstructionScript
  (|CallParentFunction))

(fn Shoot
  (bind _abilities (Variables|Abilities|GetAbilities))
  (bind (_value _returnvalue) (Utilities|Map|Find _abilities 0))
  (Utilities|FlowControl|Sequence
    (:then_0
      (Development|PrintString (Utilities|String|Append "LogBasePlayerCharacter: " "Shoot()") true false))
    (:then_1
      (if _returnvalue
        (bind _returnvalue_2 (Class|AbilitySystemComponent|TryActivateAbility (Variables|Default|GetAbilitySystem) _value true))
        (Development|PrintString (Utilities|String|ToString(Boolean) _returnvalue_2) true false)))))

(fn IsRunForward
  (bind _charactermovement (Variables|Character|GetCharacterMovement)
    (:then
      (return (Math|Float|NearlyEqual(Float) (Math|Vector|DotProduct (Math|Vector|Normalize (Variables|/Script/Engine.MovementComponent|GetVelocity _charactermovement) 1.0) (Transformation|GetActorForwardVector)) 1.0 0.5)))
    (:else)))

(fn IsSprinting
  (bind _abilitysystem (Variables|Default|GetAbilitySystem)
    (:then
      (return (GameplayTags|HasMatchingGameplayTag _abilitysystem "(TagName=\"Status.Character.Sprinting\")")))
    (:else
      (return false))))