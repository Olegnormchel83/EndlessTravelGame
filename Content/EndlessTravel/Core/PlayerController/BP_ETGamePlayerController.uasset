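; Gameplay player controller for EndlessTravel that turns Enhanced Input actions into actions on the possessed BP_ETBasePlayerCharacter.
; BeginPlay sets game-only input, adds the IMC_ET mapping context and caches the character and its movement component.
; Move, look and jump are driven directly, with strafing blocked while sprinting.
; Shoot and sprint press and release ability system input IDs (sprint only starts when running forward), while stealth activates an ability from the character's map.
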(event Input|EnhancedActionEvents|EnhancedInputActionIA_ETMove
  (params (ActionValue :type Vector%202D%20Structure) (ElapsedSeconds :type Float%20%28double-precision%29) (TriggeredSeconds :type Float%20%28double-precision%29) (InputAction :type Input%20Action%20Object%20Reference :default "/Game/EndlessTravel/Core/EnhancedInput/Actions/IA_ETMove.IA_ETMove"))
  (bind _returnvalue (Pawn|GetControlRotation :!class /Script/Engine.Controller))
  (bind _character_movement (Variables|Default|GetCharacter%20Movement)
    (:then
      (Utilities|FlowControl|Sequence
        (:then_0
          ;[1 1 1] Move Fwd/Bwd
          (Class|PawnMovementComponent|AddInputVector _character_movement (* (.y ActionValue) (Math|Vector|GetForwardVector (Math|Rotator|MakeRotator 0.0 0.0 (.yaw _returnvalue)))) false))
        (:then_1
          (if (not (Default|IsSprinting (Variables|Default|GetETBase%20Player%20Character)))
            ;[1 1 1] Move Lft/Rt
            (Class|PawnMovementComponent|AddInputVector _character_movement (* (.x ActionValue) (Math|Vector|GetRightVector (Math|Rotator|MakeRotator (.roll _returnvalue) 0.0 (.yaw _returnvalue)))) false)))))
    (:else)))

(event Input|EnhancedActionEvents|EnhancedInputActionIA_ETLook
  (params (ActionValue :type Vector%202D%20Structure) (ElapsedSeconds :type Float%20%28double-precision%29) (TriggeredSeconds :type Float%20%28double-precision%29) (InputAction :type Input%20Action%20Object%20Reference :default "/Game/EndlessTravel/Core/EnhancedInput/Actions/IA_ETLook.IA_ETLook"))
  (Class|PlayerController|AddYawInput (.x ActionValue))
  (Class|PlayerController|AddPitchInput (.y ActionValue)))

(event Input|EnhancedActionEvents|EnhancedInputActionIA_ETJump
  (params (ActionValue :type Boolean) (ElapsedSeconds :type Float%20%28double-precision%29) (TriggeredSeconds :type Float%20%28double-precision%29) (InputAction :type Input%20Action%20Object%20Reference :default "/Game/EndlessTravel/Core/EnhancedInput/Actions/IA_ETJump.IA_ETJump"))
  (:Triggered
    (bind _etbase_player_character (Variables|Default|GetETBase%20Player%20Character)
      (:then
        (Character|Jump _etbase_player_character))
      (:else)))
  (:Completed
    (bind _etbase_player_character_2 (Variables|Default|GetETBase%20Player%20Character)
      (:then
        (Character|StopJumping _etbase_player_character_2))
      (:else))))

(event Input|EnhancedActionEvents|EnhancedInputActionIA_ETShoot
  (params (ActionValue :type Boolean) (ElapsedSeconds :type Float%20%28double-precision%29) (TriggeredSeconds :type Float%20%28double-precision%29) (InputAction :type Input%20Action%20Object%20Reference :default "/Game/EndlessTravel/Core/EnhancedInput/Actions/IA_ETShoot.IA_ETShoot"))
  (:Started
    (bind _etbase_player_character (Variables|Default|GetETBase%20Player%20Character)
      (:then
        (Class|AbilitySystemComponent|PressInputID (Variables|/Game/EndlessTravel/Blueprints/Characters/PlayerCharacters/BP_ETBasePlayerCharacter.BP_ETBasePlayerCharacter_C|GetAbilitySystem _etbase_player_character) 1))
      (:else)))
  (:Completed
    (bind _etbase_player_character_2 (Variables|Default|GetETBase%20Player%20Character)
      (:then
        (Class|AbilitySystemComponent|ReleaseInputID (Variables|/Game/EndlessTravel/Blueprints/Characters/PlayerCharacters/BP_ETBasePlayerCharacter.BP_ETBasePlayerCharacter_C|GetAbilitySystem _etbase_player_character_2) 1))
      (:else))))

(event Input|EnhancedActionEvents|EnhancedInputActionIA_ETSprint
  (params (ActionValue :type Boolean) (ElapsedSeconds :type Float%20%28double-precision%29) (TriggeredSeconds :type Float%20%28double-precision%29) (InputAction :type Input%20Action%20Object%20Reference :default "/Game/EndlessTravel/Core/EnhancedInput/Actions/IA_ETSprint.IA_ETSprint"))
  (:Started
    (bind _etbase_player_character (Variables|Default|GetETBase%20Player%20Character)
      (:then
        (if (Default|IsRunForward _etbase_player_character)
          (Class|AbilitySystemComponent|PressInputID (Variables|/Game/EndlessTravel/Blueprints/Characters/PlayerCharacters/BP_ETBasePlayerCharacter.BP_ETBasePlayerCharacter_C|GetAbilitySystem _etbase_player_character) 2)))
      (:else)))
  (:Completed
    (bind _etbase_player_character_2 (Variables|Default|GetETBase%20Player%20Character)
      (:then
        (Class|AbilitySystemComponent|ReleaseInputID (Variables|/Game/EndlessTravel/Blueprints/Characters/PlayerCharacters/BP_ETBasePlayerCharacter.BP_ETBasePlayerCharacter_C|GetAbilitySystem _etbase_player_character_2) 2))
      (:else))))

(event Input|EnhancedActionEvents|EnhancedInputActionIA_ETStealth
  (params (ActionValue :type Boolean) (ElapsedSeconds :type Float%20%28double-precision%29) (TriggeredSeconds :type Float%20%28double-precision%29) (InputAction :type Input%20Action%20Object%20Reference :default "/Game/EndlessTravel/Core/EnhancedInput/Actions/IA_ETStealth.IA_ETStealth"))
  (:Started
    (bind _etbase_player_character (Variables|Default|GetETBase%20Player%20Character)
      (:then
        (if (.ReturnValue (Utilities|Map|Find (Variables|/Game/EndlessTravel/Blueprints/Characters/PlayerCharacters/BP_ETBasePlayerCharacter.BP_ETBasePlayerCharacter_C|GetAbilities _etbase_player_character) 2))
          (Class|AbilitySystemComponent|TryActivateAbility (Variables|/Game/EndlessTravel/Blueprints/Characters/PlayerCharacters/BP_ETBasePlayerCharacter.BP_ETBasePlayerCharacter_C|GetAbilitySystem _etbase_player_character) (.Value (Utilities|Map|Find (Variables|/Game/EndlessTravel/Blueprints/Characters/PlayerCharacters/BP_ETBasePlayerCharacter.BP_ETBasePlayerCharacter_C|GetAbilities _etbase_player_character) 2)) true)))
      (:else))))

(event EventBeginPlay
  (Input|SetInputModeGameOnly self false)
  (Variables|Default|SetbShowMouseCursor false)
  (Input|AddMappingContext (PlayerController|LocalPlayerSubsystems|GetEnhancedInputLocalPlayerSubsystem) "/Game/EndlessTravel/Core/EnhancedInput/IMC_ET.IMC_ET" 0 "(bIgnoreAllPressedKeysUntilRelease=True,bForceImmediately=False,bNotifyUserSettings=False)")
  (bind _asbp_etbase_player_character (Utilities|Casting|CastToBP_ETBasePlayerCharacter (Pawn|GetControlledPawn)))
  (bind _output_get (Variables|Default|SetETBase%20Player%20Character _asbp_etbase_player_character))
  (Variables|Default|SetCharacter%20Movement (Variables|/Script/Engine.Character|GetCharacterMovement _output_get)))

(fn ConstructionScript)