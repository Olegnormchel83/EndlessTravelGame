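; Game mode for EndlessTravel that manages the player's death and respawn cycle.
; It caches the first player controller and its possessed character, then listens for that character's death.
; Death broadcasts an event, switches to UI-only input with a visible cursor, and unbinds the listener.
; Reborn restarts the player, restores game input, broadcasts the respawn, and rebinds death on the refreshed character.
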(event Custom|OnPlayerDead_Event
  (Default|CallOnPlayerDead)
  (bind _etgame_player_controller (Variables|Default|GetETGame%20Player%20Controller)
    (:then
      (Input|SetInputModeUIOnly _etgame_player_controller 0 "DoNotLock" false)
      (Variables|/Script/Engine.PlayerController|SetbShowMouseCursor _etgame_player_controller true)
      (bind _etbase_player_character (Variables|Default|GetETBase%20Player%20Character)
        (:then
          (EventDispatchers|UnbindallEventsfromOnPlayerDeath _etbase_player_character))
        (:else)))
    (:else)))

(event Custom|Reborn
  (bind _etgame_player_controller (Variables|Default|GetETGame%20Player%20Controller))
  (bind _etgame_player_controller_2 (Variables|Default|GetETGame%20Player%20Controller)
    (:then
      (Class|GameModeBase|RestartPlayer _etgame_player_controller_2)
      (Input|SetInputModeGameOnly _etgame_player_controller false)
      (Variables|/Script/Engine.PlayerController|SetbShowMouseCursor _etgame_player_controller false)
      (Default|CallOnPlayerReborn)
      (bind _currentplayer (CallFunction|UpdateRefs))
      (EventDispatchers|BindEventtoOnPlayerDeath _currentplayer (EventDispatchers|CreateEvent :!event Custom|OnPlayerDead_Event)))
    (:else)))

(event EventBeginPlay
  (bind _currentplayer (CallFunction|UpdateRefs))
  (Utilities|IsValid _currentplayer
    (:Is%20Valid
      (EventDispatchers|BindEventtoOnPlayerDeath _currentplayer (delegate Custom|OnPlayerDead_Event)))))

(fn ConstructionScript)

(fn UpdateRefs
  (bind _asbp_etgame_player_controller (Utilities|Casting|CastToBP_ETGamePlayerController (Game|GetPlayerController 0))
    (:then
      (bind _output_get (Variables|Default|SetETGame%20Player%20Controller _asbp_etgame_player_controller))
      (bind _output_get_2 (Variables|Default|SetETBase%20Player%20Character (Default|GetPossesedChar _output_get)))
      (return _output_get_2))
    (:CastFailed
      (return 0))))