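; HUD for the EndlessTravel game that manages the player interface and the death screen.
; On BeginPlay it caches the game controller and game mode, binds to the game mode's player death and reborn events, then creates the interface widget for the controller's possessed character.
; On death it shows a death screen linked to the game mode and removes the interface.
; On rebirth it creates a fresh interface widget.
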(event Custom|OnPlayerReborn_Event
  (CallFunction|CreateGameInterface))

(event Custom|CreateGameInterface
  (bind _etgame_player_controller (Variables|Default|GetETGame%20Player%20Controller)
    (:then
      (bind _returnvalue (UserInterface|CreateWidget "/Game/EndlessTravel/UI/WBP_ETPlayerInterfaceTest.WBP_ETPlayerInterfaceTest_C" 0 (Default|GetPossesedChar _etgame_player_controller)))
      (bind _output_get (Variables|Default|SetETPlayerInterface _returnvalue))
      (UserInterface|Viewport|AddtoViewport _output_get 0))
    (:else)))

(event EventBeginPlay
  (Utilities|FlowControl|Sequence
    (:then_0
      (bind _asbp_etgame_player_controller (Utilities|Casting|CastToBP_ETGamePlayerController (Game|GetPlayerController 0)))
      (Variables|Default|SetETGame%20Player%20Controller _asbp_etgame_player_controller)
      (bind _asbp_etgame_game_mode (Utilities|Casting|CastToBP_ETGameGameMode (Game|GetGameMode)))
      (bind _output_get (Variables|Default|SetETGame%20Game%20Mode _asbp_etgame_game_mode))
      (EventDispatchers|BindEventtoOnPlayerDead _output_get (EventDispatchers|CreateEvent :!event OnPlayerDeadFunc))
      (EventDispatchers|BindEventtoOnPlayerReborn _output_get (delegate Custom|OnPlayerReborn_Event)))
    (:then_1
      (CallFunction|CreateGameInterface))))

(event Collision|EventActorBeginOverlap
  (params (OtherActor :type Actor%20Object%20Reference)))

(event EventTick
  (params (DeltaSeconds :type Float%20%28single-precision%29)))

(fn ConstructionScript)

(fn OnPlayerDeadFunc
  (bind _returnvalue (UserInterface|CreateWidget "/Game/EndlessTravel/UI/WBP_DeadScreen.WBP_DeadScreen_C" 0 (Variables|Default|GetETGame%20Game%20Mode)))
  (bind _output_get (Variables|Default|SetETDeathScreen _returnvalue))
  (UserInterface|Viewport|AddtoViewport _output_get 0)
  (bind _etplayerinterface (Variables|Default|GetETPlayerInterface)
    (:then
      (Widget|RemovefromParent _etplayerinterface))
    (:else)))